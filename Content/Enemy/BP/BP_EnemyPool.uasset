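; Object pool for Enemy_Soldier actors that reuses inactive soldiers.
; On BeginPlay it pre-spawns deactivated soldiers at the EnemySpawner's transform, using InitialSize as the loop bound.
; AcquireEnemy activates and removes the last inactive soldier; if none remain, it spawns one and adds it to the inactive list without calling ActivateEnemy.
; ReleaseEnemy deactivates an enemy and returns it to the list.
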(event Collision|EventActorBeginOverlap
  (params (OtherActor :type Actor%20Object%20Reference)))

(event EventTick
  (params (DeltaSeconds :type Float%20%28single-precision%29)))

(event EventBeginPlay
  (bind _returnvalue (Actor|GetActorOfClass "/Game/Enemy/BP/EnemySpawner.EnemySpawner_C"))
  (for _index (range 0 (Variables|Default|GetInitialSize))
    (bind _returnvalue_2 (Game|SpawnActorfromClass "/Game/Enemy/BP/Enemy_Soldier.Enemy_Soldier_C" (Transformation|GetActorTransform _returnvalue) "Undefined" "MultiplyWithRoot" 0 0))
    (Default|DeactivateEnemy _returnvalue_2)
    (Utilities|Array|Add (Variables|Default|GetInactiveEnemies) _returnvalue_2)))

(fn ConstructionScript)

(fn AcquireEnemy
  (bind _inactiveenemies (Variables|Default|GetInactiveEnemies))
  (bind _inactiveenemies_2 (Variables|Default|GetInactiveEnemies))
  (if (> (Utilities|Array|Length (Variables|Default|GetInactiveEnemies)) 0)
    (Development|PrintString "pool")
    (Default|ActivateEnemy (Utilities|Array|Get(acopy) _inactiveenemies (Utilities|Array|LastIndex _inactiveenemies)))
    (Utilities|Array|RemoveIndex _inactiveenemies_2 (Utilities|Array|LastIndex _inactiveenemies_2))
    (else
      (Development|PrintString "spawn")
      (bind _returnvalue (Actor|GetActorOfClass "/Game/Enemy/BP/EnemySpawner.EnemySpawner_C"))
      (bind _returnvalue_2 (Game|SpawnActorfromClass "/Game/Enemy/BP/Enemy_Soldier.Enemy_Soldier_C" (Transformation|GetActorTransform _returnvalue) "Undefined" "MultiplyWithRoot" 0 0))
      (Utilities|Array|Add (Variables|Default|GetInactiveEnemies) _returnvalue_2))))

(fn ReleaseEnemy
  (params (Enemy :type Enemy%20Base%20Object%20Reference))
  (Default|DeactivateEnemy Enemy)
  (Utilities|Array|Add (Variables|Default|GetInactiveEnemies) Enemy))